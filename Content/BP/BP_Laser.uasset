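; BP_Laser is an actor that fires a red laser along its forward vector every tick and bounces it off reflectors.
; A visibility line trace finds the first hit, and the beam itself is rendered with debug lines.
; On a BP_Reflector hit, the beam stops there and hands the reflected direction to that reflector's ShootARay.
; Otherwise the beam draws to its full length, even through non-reflector objects.
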(event EventTick
  (params (DeltaSeconds :type Float%20%28single-precision%29))
  (CallFunction|ShootLaser))

(fn ConstructionScript)

(fn LineTrace
  (bind _returnvalue (Transformation|GetActorLocation))
  (bind (_outhit _returnvalue_2) (Collision|LineTraceByChannel _returnvalue (+ _returnvalue (* (Transformation|GetActorForwardVector) (Variables|Default|GetInfinity))) "TraceTypeQuery1" false 0 "None"))
  (return _outhit _returnvalue_2))

(fn LineDrawHit
  (params (LineStart :type Vector) (LineEnd :type Vector))
  (Rendering|Debug|DrawDebugLine LineStart LineEnd "(R=1.000000,G=0.010379,B=0.000000,A=1.000000)" 0.0 5.0))

(fn LineDrawNoHit
  (bind _returnvalue (Transformation|GetActorLocation))
  (Rendering|Debug|DrawDebugLine _returnvalue (+ _returnvalue (* (Transformation|GetActorForwardVector) (Variables|Default|GetInfinity))) "(R=1.000000,G=0.010379,B=0.000000,A=1.000000)" 0.0 5.0))

(fn ShootLaser
  (bind (_hitresult _bwasahit) (CallFunction|LineTrace))
  (LocalVariables|SetHitResult _hitresult)
  (if _bwasahit
    (bind _asbp_reflector (Utilities|Casting|CastToBP_Reflector (.HitActor (Collision|BreakHitResult (LocalVariables|GetHitResult))))
      (:then
        ;[0 0.02083 0.000596 1 25] If the object hit was a reflector aka cast was successful
        (CallFunction|LineDrawHit (.TraceStart (Collision|BreakHitResult (LocalVariables|GetHitResult))) (.Location (Collision|BreakHitResult (LocalVariables|GetHitResult))))
        (Default|ShootARay _asbp_reflector (.Location (Collision|BreakHitResult (LocalVariables|GetHitResult))) (Math|Vector|GetReflectionVector (Math|Vector|Normalize (- (.Location (Collision|BreakHitResult (LocalVariables|GetHitResult))) (.TraceStart (Collision|BreakHitResult (LocalVariables|GetHitResult))))) (.Normal (Collision|BreakHitResult (LocalVariables|GetHitResult)))) (Variables|Default|GetInfinity) self))
      (:CastFailed
        ;[0.05729 0.000584 0.001724 1 25] If a hit but not a 'reflector', still draw laser line to infinity
        (CallFunction|LineDrawNoHit)))
    (else
      ;[0.08854 0.01844 0.01932] If not a hit, draw laser line to infinity
      (CallFunction|LineDrawNoHit))))