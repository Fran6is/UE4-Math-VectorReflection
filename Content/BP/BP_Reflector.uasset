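; BP_Reflector is a mirror actor that bounces a laser ray onward through a chain of reflectors.
; ShootARay line-traces on Visibility and, on hitting another reflector, recursively calls that actor's ShootARay with the reflected direction and incremented bounce count.
; The passed-in laser's MaxBounces caps the recursion.
; Beam segments are debug lines, drawn to reflector hits or at full ray length otherwise, even through non-reflector obstacles.
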(event EventBeginPlay)

(event Collision|EventActorBeginOverlap
  (params (OtherActor :type Actor%20Object%20Reference)))

(event EventTick
  (params (DeltaSeconds :type Float%20%28single-precision%29)))

(fn ConstructionScript)

(fn ShootARay
  (params (RayOrigin :type Vector) (RayDirection :type Vector) (RayLength :type Float%20%28single-precision%29) (Laser%20Reference :type BP%20Laser%20Object%20Reference) (BounceCount :type Integer))
  ;[1 1 1] Set some local variables to use inside the function to reduce clutter
  (LocalVariables|SetTraceLength RayLength)
  (LocalVariables|SetRayOrig RayOrigin)
  (LocalVariables|SetRayDir RayDirection)
  (LocalVariables|SetLaserRef Laser%20Reference)
  (bind _output_get (LocalVariables|SetBounceCountt BounceCount))
  ;[1 1 1] Only shoot a ray if within the maximum number of bounces
  (if (<= (+ _output_get 1) (Variables|/Game/BP/BP_Laser.BP_Laser_C|GetMaxBounces (LocalVariables|GetLaserRef)))
    (bind (_outhit _returnvalue) (Collision|LineTraceByChannel RayOrigin (+ RayOrigin (* RayDirection RayLength)) "TraceTypeQuery1" false 0 "None"))
    (if _returnvalue
      (bind _asbp_reflector (Utilities|Casting|CastToBP_Reflector (.HitActor (Collision|BreakHitResult _outhit)))
        (:then
          ;[1 1 1] If a hit and the object hit is a reflector
          (Rendering|Debug|DrawDebugLine (.TraceStart (Collision|BreakHitResult _outhit)) (.Location (Collision|BreakHitResult _outhit)) "(R=1.000000,G=0.010379,B=0.000000,A=1.000000)" 0.0 5.0)
          (CallFunction|ShootARay _asbp_reflector (.Location (Collision|BreakHitResult _outhit)) (Math|Vector|GetReflectionVector (Math|Vector|Normalize (- (.Location (Collision|BreakHitResult _outhit)) (.TraceStart (Collision|BreakHitResult _outhit)))) (.Normal (Collision|BreakHitResult _outhit))) (LocalVariables|GetTraceLength) (LocalVariables|GetLaserRef) (+ (LocalVariables|GetBounceCountt) 1)))
        (:CastFailed
          ;[1 1 1] If no hit or object hit is not a reflector
          (Rendering|Debug|DrawDebugLine (LocalVariables|GetRayOrig) (+ (LocalVariables|GetRayOrig) (* (LocalVariables|GetRayDir) (LocalVariables|GetTraceLength))) "(R=1.000000,G=0.010379,B=0.000000,A=1.000000)" 0.0 5.0 :!label _label)))
      (else
        (goto _label)))))